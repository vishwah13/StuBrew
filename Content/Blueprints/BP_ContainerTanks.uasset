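; Container tank actor whose Cylinder mesh shows a liquid level that rises during play.
; The construction script applies the initial LiquidLevel, then Tick grows it in proportion to its current value and Speed until it passes a fixed cap.
; SetLiquidLevelMesh pushes the value to a material scalar parameter, calling CreateDynamicMaterialInstance on every update rather than caching the instance.
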(event EventTick
  (params (DeltaSeconds :type Float%20%28single-precision%29))
  (if (<= (Variables|Default|GetLiquidLevel) 0.8)
    (bind _output_get (Variables|Default|SetLiquidLevel (+ (Variables|Default|GetLiquidLevel) (* (Variables|Default|GetLiquidLevel) DeltaSeconds (Variables|Default|GetSpeed)))))
    (CallFunction|SetLiquidLevelMesh (Variables|Default|GetCylinder) _output_get)))

(fn ConstructionScript
  (CallFunction|SetLiquidLevelMesh (Variables|Default|GetCylinder) (Variables|Default|GetLiquidLevel)))

(fn SetLiquidLevelMesh
  (params (Target :type Primitive%20Component%20Object%20Reference) (Value :type Float%20%28single-precision%29))
  (bind _returnvalue (Rendering|Material|CreateDynamicMaterialInstance Target 0 (Rendering|Material|GetMaterial Target 0) "None" :!class /Script/Engine.PrimitiveComponent))
  (Rendering|Material|SetScalarParameterValue _returnvalue "LiquidLevel" Value :!class /Script/Engine.MaterialInstanceDynamic))