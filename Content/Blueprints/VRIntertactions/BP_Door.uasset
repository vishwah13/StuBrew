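; BP_Door is a VR door that highlights its knob while a VRPawn is inside its Box trigger.
; Every Tick, HighLightMesh polls the Box for overlapping pawns and sets the "Selected" scalar material parameter on DoorKnob on or off.
; The construction script copies the LeftHand and RightHand references into MyAttachComponent.
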(event EventTick
  (params (DeltaSeconds :type Float%20%28single-precision%29))
  (CallFunction|HighLightMesh (Variables|Default|GetDoorKnob)))

(fn ConstructionScript
  (bind _myattachcomponent (Variables|Default|GetMyAttachComponent))
  (Variables|/Game/Blueprints/VRIntertactions/MyAttachComponent.MyAttachComponent_C|SetLeftHand _myattachcomponent (Variables|Default|GetLeftHand))
  (Variables|/Game/Blueprints/VRIntertactions/MyAttachComponent.MyAttachComponent_C|SetRighthand _myattachcomponent (Variables|Default|GetRightHand)))

(fn HighLightMesh
  (params (MeshToHighlight :type Mesh%20Component%20Object%20Reference))
  (if (> (Utilities|Array|Length (Collision|GetOverlappingActors (Variables|Default|GetBox) "/Game/VRTemplate/Blueprints/VRPawn.VRPawn_C" :!class /Script/Engine.PrimitiveComponent)) 0)
    (Rendering|Material|SetScalarParameterValueonMaterials MeshToHighlight "Selected" 1.0)
    (else
      (Rendering|Material|SetScalarParameterValueonMaterials MeshToHighlight "Selected" 0.0))))