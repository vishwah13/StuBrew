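; BP_Button is a VR push button that sinks while a VRPawn overlaps its collision box and rises back when the overlap ends.
; Each Tick polls the box and steps the Button component's relative Z through near-instant MoveComponentTo calls, clamped between zero and ButtonOffset.
; The construction script uses ButtonOffset to set both the raised rest height and the Arrow's length.
; The graph only moves the button and triggers no press event.
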(event EventTick
  (params (DeltaSeconds :type Float%20%28single-precision%29))
  (bind _button (Variables|Default|GetButton))
  (bind _button_2 (Variables|Default|GetButton))
  (if (> (Utilities|Array|Length (Collision|GetOverlappingActors (Variables|Default|GetBoxCollision) "/Game/VRTemplate/Blueprints/VRPawn.VRPawn_C" :!class /Script/Engine.PrimitiveComponent)) 0)
    (Components|MoveComponentTo _button_2 (Math|Vector|MakeVector 0.0 0.0 (Math|Float|Clamp(Float) (- (.z (Variables|/Script/Engine.SceneComponent|GetRelativeLocation _button_2)) 3.0) 0.0 (Variables|Default|GetButtonOffset))) "0, 0, 0" false false 0.0001 false)
    (else
      (Components|MoveComponentTo _button (Math|Vector|MakeVector 0.0 0.0 (Math|Float|Clamp(Float) (+ (.z (Variables|/Script/Engine.SceneComponent|GetRelativeLocation _button)) 3.0) 0.0 (Variables|Default|GetButtonOffset))) "0, 0, 0" false false 0.0001 false))))

(fn ConstructionScript
  (bind _buttonoffset (Variables|Default|GetButtonOffset))
  (Variables|/Script/Engine.ArrowComponent|SetArrowLength (Variables|Default|GetArrow) _buttonoffset)
  (Transformation|SetRelativeLocation (Variables|Default|GetButton) (Math|Vector|MakeVector 0.0 0.0 _buttonoffset) false false))