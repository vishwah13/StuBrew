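; BP_Containers is a grabbable VR container that emits pouring-style particles when tipped while held.
; Each tick, it checks the holding motion controller's relative roll and pitch, raising the NSFX spawn rate beyond a tilt threshold in either direction and zeroing it otherwise.
; HighLightMesh also runs every tick, setting the cylinder material's Selected parameter when a VRPawn overlaps the box and the container is not held.
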(event EventTick
  (params (DeltaSeconds :type Float%20%28single-precision%29))
  (bind _grabcomponent (Variables|Default|GetGrabComponent))
  (CallFunction|HighLightMesh (Variables|Default|GetCylinder))
  (if (Variables|/Game/VRTemplate/Blueprints/GrabComponent.GrabComponent_C|GetbIsHeld _grabcomponent)
    (bind _motioncontrollerref (Variables|/Game/VRTemplate/Blueprints/GrabComponent.GrabComponent_C|GetMotionControllerRef _grabcomponent)
      (:then
        (if (Math|Boolean|ORBoolean (> (.roll (Variables|/Script/Engine.SceneComponent|GetRelativeRotation _motioncontrollerref)) 1.2e+02) (> (.pitch (Variables|/Script/Engine.SceneComponent|GetRelativeRotation _motioncontrollerref)) 1.2e+02) (< (.roll (Variables|/Script/Engine.SceneComponent|GetRelativeRotation _motioncontrollerref)) -1.2e+02) (< (.pitch (Variables|/Script/Engine.SceneComponent|GetRelativeRotation _motioncontrollerref)) -1.2e+02))
          (Effects|Components|ParticleSystem|SetFloatParameter (Variables|Default|GetNS_FX) "User.SpawnRate" 5e+01)
          (else
            (Effects|Components|ParticleSystem|SetFloatParameter (Variables|Default|GetNS_FX) "User.SpawnRate" 0.0))))
      (:else))))

(fn ConstructionScript
  (Effects|Components|ParticleSystem|SetFloatParameter (Variables|Default|GetNS_FX) "User.SpawnRate" 0.0))

(fn HighLightMesh
  (params (MeshToHighlight :type Mesh%20Component%20Object%20Reference))
  (if (Variables|/Game/VRTemplate/Blueprints/GrabComponent.GrabComponent_C|GetbIsHeld (Variables|Default|GetGrabComponent))
    (Rendering|Material|SetScalarParameterValueonMaterials MeshToHighlight "Selected" 0.0)
    (elif (> (Utilities|Array|Length (Collision|GetOverlappingActors (Variables|Default|GetBox) "/Game/VRTemplate/Blueprints/VRPawn.VRPawn_C" :!class /Script/Engine.PrimitiveComponent)) 0)
      (Rendering|Material|SetScalarParameterValueonMaterials MeshToHighlight "Selected" 1.0)
      (else
        (Rendering|Material|SetScalarParameterValueonMaterials MeshToHighlight "Selected" 0.0)))))