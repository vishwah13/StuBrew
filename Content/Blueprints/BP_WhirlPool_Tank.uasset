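; Whirlpool tank actor for a VR game that spins its whirlpool and tracks a water level held by the game mode.
; Each Tick runs the parent logic, then yaws the spin cylinder at a configurable, frame-rate-independent speed.
; It also polls VRGameMode and copies the water level into LiquidLevel only within a fixed range, otherwise keeping the last value.
; Nothing in this graph consumes LiquidLevel.
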(event EventBeginPlay)

(event Collision|EventActorBeginOverlap
  (params (OtherActor :type Actor%20Object%20Reference)))

(event EventTick
  (params (DeltaSeconds :type Float%20%28single-precision%29))
  (|CallParentFunction DeltaSeconds)
  (Transformation|AddWorldRotation (Variables|Default|GetWhirlPoolParts_WhirlpoolSpinCylinder) (Math|Rotator|MakeRotator 0.0 0.0 (* DeltaSeconds (Variables|Default|GetWhirlPoolRotationSpeed))) false false)
  (bind _asvrgame_mode (Utilities|Casting|CastToVRGameMode (Game|GetGameMode))
    (:then
      (if (and (>= (Variables|/Game/VRTemplate/Blueprints/VRGameMode.VRGameMode_C|GetWhirlPoolWaterLevel _asvrgame_mode) 0.2) (<= (Variables|/Game/VRTemplate/Blueprints/VRGameMode.VRGameMode_C|GetWhirlPoolWaterLevel _asvrgame_mode) 0.9))
        (Variables|Default|SetLiquidLevel (Variables|/Game/VRTemplate/Blueprints/VRGameMode.VRGameMode_C|GetWhirlPoolWaterLevel _asvrgame_mode))))
    (:CastFailed
      (Development|PrintString "VR GameMode CAST FAILD !!"))))

(fn ConstructionScript
  (|CallParentFunction))