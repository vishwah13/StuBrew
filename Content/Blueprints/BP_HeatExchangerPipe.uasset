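; BP_HeatExchangerPipe is a VR heat exchanger pipe that changes color after the kettle starts.
; BeginPlay caches the VRGameMode, and Tick polls its StartKettle flag.
; While the flag is set, Tick waits TimeToChangeColor through a Delay, then ChangeColor sets the BaseColor vector parameter on the Pipe materials to Color.
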(event EventTick
  (params (DeltaSeconds :type Float%20%28single-precision%29))
  (if (Variables|/Game/VRTemplate/Blueprints/VRGameMode.VRGameMode_C|GetStartKettle (Variables|Default|GetAs%20VRGame%20Mode))
    (Utilities|FlowControl|Delay (Variables|Color|GettimeToChangeColor))
    (CallFunction|ChangeColor (Variables|Color|GetColor))))

(event EventBeginPlay
  (bind _asvrgame_mode (Utilities|Casting|CastToVRGameMode (Game|GetGameMode)))
  (Variables|Default|SetAs%20VRGame%20Mode _asvrgame_mode))

(fn ConstructionScript)

(fn ChangeColor
  (params (ParameterValue :type Vector))
  (Rendering|Material|SetVectorParameterValueonMaterials (Variables|Default|GetPipe) "BaseColor" ParameterValue))