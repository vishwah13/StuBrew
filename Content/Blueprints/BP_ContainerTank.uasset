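; BP_ContainerTank is a brewery container tank that displays its liquid level through a material parameter on its middle cylinder mesh.
; The construction script calls SetLiquidLevelMesh, which creates a dynamic material instance from slot 0 and sets its LiquidLevel scalar.
; A gradual fill driven by Speed exists in the event graph but is disconnected from Tick, so the level stays static at runtime.
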(event EventTick
  (params (DeltaSeconds :type Float%20%28single-precision%29)))

(fn ConstructionScript
  (CallFunction|SetLiquidLevelMesh (Variables|Default|GetMyBrewery_Mid_Cylinder) (Variables|Default|GetLiquidLevel)))

(fn SetLiquidLevelMesh
  (params (Target :type Primitive%20Component%20Object%20Reference) (Value :type Float%20%28single-precision%29))
  (bind _returnvalue (Rendering|Material|CreateDynamicMaterialInstance Target 0 (Rendering|Material|GetMaterial Target 0) "None" :!class /Script/Engine.PrimitiveComponent))
  (Rendering|Material|SetScalarParameterValue _returnvalue "LiquidLevel" Value :!class /Script/Engine.MaterialInstanceDynamic))