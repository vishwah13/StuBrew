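; Brewery whirlpool button that switches the whirlpool on through VRGameMode's StartWirlPool flag.
; Tick polls IsPressed, which is not set in this graph; when true, it raises the flag, plays a 2D sound and clears the press.
; While unpressed, Tick keeps feeding a six-second Delay that lowers the flag, so shutoff follows that repeating timer and can come sooner after a press.
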(event EventBeginPlay
  (bind _asvrgame_mode (Utilities|Casting|CastToVRGameMode (Game|GetGameMode)))
  (Variables|Default|SetAs%20VRGame%20Mode _asvrgame_mode))

(event EventTick
  (params (DeltaSeconds :type Float%20%28single-precision%29))
  (|CallParentFunction DeltaSeconds)
  (Utilities|FlowControl|Sequence
    (:then_0
      (if (Variables|Default|GetIsPressed?)
        (Variables|/Game/VRTemplate/Blueprints/VRGameMode.VRGameMode_C|SetStartWirlPool (Variables|Default|GetAs%20VRGame%20Mode) true)
        (bind _returnvalue (Audio|SpawnSound2D "/Game/StarterContent/Audio/Smoke01.Smoke01" 1.0 1.0 0.0 0))
        (Variables|Default|SetWhirlPoolSound _returnvalue)
        (Variables|Default|SetIsPressed? false)))
    (:then_1
      (if (not (Variables|Default|GetIsPressed?))
        (Utilities|FlowControl|Delay 6.0)
        (Variables|/Game/VRTemplate/Blueprints/VRGameMode.VRGameMode_C|SetStartWirlPool (Variables|Default|GetAs%20VRGame%20Mode) false)))))

(fn ConstructionScript
  (|CallParentFunction))