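; Mash tun button for the VR brewery that starts the mashing step and updates the player's objective.
; Tick polls IsPressed, then sets StartMashTun on the VRGameMode, plays a smoke sound, clears the press and sets a one-time wait objective.
; While unpressed, a two-second Delay driven from Tick stops any valid mash sound and sets a one-time objective to pull the mash lever.
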(event EventBeginPlay
  (bind _asvrgame_mode (Utilities|Casting|CastToVRGameMode (Game|GetGameMode)))
  (Variables|Default|SetAs%20VRGame%20Mode _asvrgame_mode))

(event EventTick
  (params (DeltaSeconds :type Float%20%28single-precision%29))
  (|CallParentFunction DeltaSeconds)
  (Utilities|FlowControl|Sequence
    (:then_0
      (if (Variables|Default|GetIsPressed?)
        (Variables|/Game/VRTemplate/Blueprints/VRGameMode.VRGameMode_C|SetStartMashTun (Variables|Default|GetAs%20VRGame%20Mode) true)
        (bind _returnvalue (Audio|SpawnSound2D "/Game/StarterContent/Audio/Smoke01.Smoke01" 1.0 1.0 0.0 0))
        (Variables|Default|SetMashSound _returnvalue)
        (Variables|Default|SetIsPressed? false)
        (Utilities|FlowControl|DoOnce false
          (:Completed
            (CallFunction|SetObjective "Wait For Mashing to finish")))))
    (:then_1
      (if (not (Variables|Default|GetIsPressed?))
        (Utilities|FlowControl|Delay 2.0)
        (Utilities|IsValid (Variables|Default|GetMashSound)
          (:Is%20Valid
            (Audio|Components|Audio|Stop (Variables|Default|GetMashSound))
            (Utilities|FlowControl|DoOnce false
              (:Completed
                (CallFunction|SetObjective "Pull The Mash Lever !")))))))))

(fn ConstructionScript
  (|CallParentFunction))