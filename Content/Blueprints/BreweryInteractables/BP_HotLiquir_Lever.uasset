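; BP_HotLiquir_Lever is a brewery lever that drains the hot water container and fills the mash tun while pulled.
; Each tick it checks the attach component's IsPulled flag and edits both water levels stored on the cached VRGameMode.
; Each change scales with delta time, its own speed and that vessel's current level, so the rates are exponential and an empty mash tun stays empty.
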(event EventBeginPlay
  (|CallParentFunction)
  (bind _asvrgame_mode (Utilities|Casting|CastToVRGameMode (Game|GetGameMode)))
  (Variables|Default|SetAs%20VRGame%20Mode _asvrgame_mode))

(event Collision|EventActorBeginOverlap
  (params (OtherActor :type Actor%20Object%20Reference))
  (|CallParentFunction OtherActor) ; This node is disabled and will not be called.\nDrag off pins to build functionality.
)

(event EventTick
  (params (DeltaSeconds :type Float%20%28single-precision%29))
  (bind _as_vrgame_mode (Variables|Default|GetAs%20VRGame%20Mode))
  (|CallParentFunction DeltaSeconds)
  (if (Variables|/Game/Blueprints/VRIntertactions/MyAttachComponent.MyAttachComponent_C|GetbIsPulled? (Variables|Default|GetMyAttachComponent))
    (Variables|/Game/VRTemplate/Blueprints/VRGameMode.VRGameMode_C|SetHotWaterContainerLevel _as_vrgame_mode (- (Variables|/Game/VRTemplate/Blueprints/VRGameMode.VRGameMode_C|GetHotWaterContainerLevel _as_vrgame_mode) (* (Utilities|Time|GetWorldDeltaSeconds) (Variables|Default|GetDrainSpeed) (Variables|/Game/VRTemplate/Blueprints/VRGameMode.VRGameMode_C|GetHotWaterContainerLevel _as_vrgame_mode))))
    (Variables|/Game/VRTemplate/Blueprints/VRGameMode.VRGameMode_C|SetMashTunWaterLevel _as_vrgame_mode (+ (Variables|/Game/VRTemplate/Blueprints/VRGameMode.VRGameMode_C|GetMashTunWaterLevel _as_vrgame_mode) (* (Utilities|Time|GetWorldDeltaSeconds) (Variables|Default|GetMashTunFillSpeed) (Variables|/Game/VRTemplate/Blueprints/VRGameMode.VRGameMode_C|GetMashTunWaterLevel _as_vrgame_mode))))))

(fn ConstructionScript
  (|CallParentFunction))