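; Brewery hot liquor button that, once pressed, heats the liquor toward a target temperature and guides the player through objectives.
; Tick eases the temperature up with FInterpTo, shows it rounded on a text render, and prompts the player to wait.
; It spawns a low-pitched sound every heating tick, keeping only the latest reference.
; Near the target, it stops that sound and sets the lever-pull objective once.
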(event EventBeginPlay)

(event Collision|EventActorBeginOverlap
  (params (OtherActor :type Actor%20Object%20Reference)))

(event EventTick
  (params (DeltaSeconds :type Float%20%28single-precision%29))
  (|CallParentFunction DeltaSeconds)
  (Utilities|FlowControl|Sequence
    (:then_0
      (if (and (Variables|Default|GetIsPressed?) (!= (Variables|Default|GetHotLiquorTemp) 77.0))
        (bind _returnvalue (Audio|SpawnSoundatLocation "/Game/StarterContent/Audio/Smoke01.Smoke01" (Transformation|GetActorLocation) "0, 0, 0" 1.0 0.1 0.0 0 0))
        (Variables|Default|SetHeatSound _returnvalue)
        (Variables|Default|SetHotLiquorTemp (Math|Interpolation|FInterpTo (Variables|Default|GetHotLiquorTemp) 77.0 DeltaSeconds 0.5))
        (Rendering|Components|TextRender|SetText (Variables|/Script/Engine.TextRenderActor|GetTextRender (Variables|Default|GetHotLiquorTemp_Text)) (Utilities|Text|ToText(String) (Utilities|String|Append (Utilities|String|ToString(Float) (Math|Conversions|ToFloat(Integer) (Math|Float|Round (Math|Interpolation|FInterpTo (Variables|Default|GetHotLiquorTemp) 77.0 DeltaSeconds 0.5)))) "°C")))
        (Utilities|FlowControl|DoOnce false
          (:Completed
            (CallFunction|SetObjective "Wait for the Temprature to raise to 77 degrees")))))
    (:then_1
      (if (>= (Variables|Default|GetHotLiquorTemp) 76.0)
        (Utilities|IsValid (Variables|Default|GetHeatSound)
          (:Is%20Valid
            (Audio|Components|Audio|Stop (Variables|Default|GetHeatSound))
            (Utilities|FlowControl|DoOnce false
              (:Completed
                (CallFunction|SetObjective "Pull The Lever !")))))))))

(fn ConstructionScript
  (|CallParentFunction))