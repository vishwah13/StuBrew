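; BP_Kettle_Button is an interactable brewery button that starts the kettle in the VR game mode.
; It caches the VRGameMode on BeginPlay, then polls IsPressed each Tick after calling the parent Tick.
; When pressed, it sets StartKettle on the game mode, spawns the Smoke01 2D sound, stores it as KettleSound and clears IsPressed.
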(event EventBeginPlay
  (bind _asvrgame_mode (Utilities|Casting|CastToVRGameMode (Game|GetGameMode)))
  (Variables|Default|SetAs%20VRGame%20Mode _asvrgame_mode))

(event EventTick
  (params (DeltaSeconds :type Float%20%28single-precision%29))
  (|CallParentFunction DeltaSeconds)
  (if (Variables|Default|GetIsPressed?)
    (Variables|/Game/VRTemplate/Blueprints/VRGameMode.VRGameMode_C|SetStartKettle (Variables|Default|GetAs%20VRGame%20Mode) true)
    (bind _returnvalue (Audio|SpawnSound2D "/Game/StarterContent/Audio/Smoke01.Smoke01" 1.0 1.0 0.0 0))
    (Variables|Default|SetKettleSound _returnvalue)
    (Variables|Default|SetIsPressed? false)))

(fn ConstructionScript
  (|CallParentFunction))