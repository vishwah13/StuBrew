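; BP_HotLiquirTank is a hot liquid tank whose level follows the hot water container level stored in VRGameMode.
; Each Tick runs the parent logic, then copies that level into LiquidLevel once it reaches a minimum threshold, printing an error if the game mode cast fails.
; When LiquidLevel reaches a higher fill threshold, a DoOnce sets the objective prompting the player to push the button.
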(event EventBeginPlay)

(event Collision|EventActorBeginOverlap
  (params (OtherActor :type Actor%20Object%20Reference)))

(event EventTick
  (params (DeltaSeconds :type Float%20%28single-precision%29))
  (|CallParentFunction DeltaSeconds)
  (bind _asvrgame_mode (Utilities|Casting|CastToVRGameMode (Game|GetGameMode))
    (:then
      (if (>= (Variables|/Game/VRTemplate/Blueprints/VRGameMode.VRGameMode_C|GetHotWaterContainerLevel _asvrgame_mode) 0.2)
        (bind _output_get (Variables|Default|SetLiquidLevel (Variables|/Game/VRTemplate/Blueprints/VRGameMode.VRGameMode_C|GetHotWaterContainerLevel _asvrgame_mode)))
        (if (>= _output_get 0.7)
          (Utilities|FlowControl|DoOnce false
            (:Completed
              (CallFunction|SetObjective "Push The Button !"))))))
    (:CastFailed
      (Development|PrintString "VR GameMode CAST FAILD !!"))))

(fn ConstructionScript
  (|CallParentFunction))